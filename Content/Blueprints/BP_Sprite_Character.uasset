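; BP_Sprite_Character is a Paper2D player character with sideways movement and run or idle flipbook animation.
; The MoveRight input axis feeds AddMovementInput along world X.
; UpdateAnimation picks the run or idle flipbook from whether movement velocity is non-zero, but only BeginPlay calls it, as Tick is disabled.
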(event Custom|UpdateAnimation
  (Sprite|SetFlipbook (Variables|Default|GetSprite) (select (> (Math|Vector|VectorLength (Variables|/Script/Engine.MovementComponent|GetVelocity (Variables|Character|GetCharacterMovement))) 0.0) "/Game/SunnyLandAssets/sprites/player/run/FB_Player_Run.FB_Player_Run" "/Game/SunnyLandAssets/sprites/player/idle/FB_Player_Idle.FB_Player_Idle")))

(event EventBeginPlay
  (CallFunction|UpdateAnimation))

(event Collision|EventActorBeginOverlap
  (params (OtherActor :type Actor%20Object%20Reference)))

(event EventTick
  (params (DeltaSeconds :type Float%20%28single-precision%29)))

(event Input|AxisEvents|InputAxisMoveRight
  (params (AxisValue :type Float%20%28single-precision%29))
  (Pawn|Input|AddMovementInput "1.000000, 0, 0" AxisValue false))

(fn ConstructionScript)